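; Sword weapon Blueprint that moves between a holster socket and an equipped socket, with a dissolve material effect.
; BeginPlay creates a dynamic dissolve material instance on the mesh and attaches the sword to SwordHolster.
; OnEquip attaches it to the Sword socket.
; OnUnequip returns it to the holster and plays a timeline that drives the material's Amount parameter; equipping does not animate it.
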(event EventBeginPlay
  (bind _returnvalue (Rendering|Material|CreateDynamicMaterialInstance (Variables|Default|GetMesh) 0 "/Game/Material/MAT_WeaponDissolve_Inst.MAT_WeaponDissolve_Inst" "None" :!class /Script/Engine.PrimitiveComponent))
  (Variables|Default|SetDynamic%20Material _returnvalue)
  (Class|CAttachment|Attachto "SwordHolster"))

(event EventOnEquip
  (Class|CAttachment|Attachto "Sword"))

(event EventOnUnequip
  (Class|CAttachment|Attachto "SwordHolster")
  (bind _output (Timeline|타임라인 PlayFromStart)
    (:Update
      (Rendering|Material|SetScalarParameterValue (Variables|Default|GetDynamic%20Material) "Amount" _output :!class /Script/Engine.MaterialInstanceDynamic))))

(fn ConstructionScript)