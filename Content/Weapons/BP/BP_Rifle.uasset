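; Rifle weapon Blueprint that moves between a holster and an equipped attach point as it is equipped and unequipped.
; On BeginPlay it creates a dynamic instance of M_KA47 on its skeletal mesh and attaches to RifleHolster.
; OnEquip attaches it to Rifle; OnUnequip returns it to RifleHolster and plays a timeline that animates the material's Amount parameter.
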(event EventBeginPlay
  (bind _returnvalue (Rendering|Material|CreateDynamicMaterialInstance (Variables|Default|GetSkeletalMesh) 0 "/Game/Weapons/FPS_Weapon_Bundle/Weapons/Materials/Ka47/M_KA47.M_KA47" "None" :!class /Script/Engine.PrimitiveComponent))
  (Variables|Default|SetDynamicMaterial _returnvalue)
  (Class|CAttachment|Attachto "RifleHolster"))

(event Collision|EventActorBeginOverlap
  (params (OtherActor :type Actor%20Object%20Reference)))

(event EventTick
  (params (DeltaSeconds :type Float%20%28single-precision%29)))

(event EventOnEquip
  (Class|CAttachment|Attachto "Rifle"))

(event EventOnUnequip
  (Class|CAttachment|Attachto "RifleHolster")
  (bind _output (Timeline|타임라인 PlayFromStart)
    (:Update
      (Rendering|Material|SetScalarParameterValue (Variables|Default|GetDynamicMaterial) "Amount" _output :!class /Script/Engine.MaterialInstanceDynamic))))

(fn ConstructionScript)